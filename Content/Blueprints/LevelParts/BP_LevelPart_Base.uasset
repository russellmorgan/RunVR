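; Base Blueprint for a level part in a chain of parts that spawn as the player progresses.
; When the player overlaps LevelPassTrigger, it has BP_GameMode add another part and increase the score, then destroys itself after a short delay.
; FindAttachPoint returns the world transform of the AttachPoint at the part's end.
; The construction script adds a child actor at EnemySpawnPoint's relative location.
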(event `self.LevelPassTrigger.OnComponentBeginOverlap`
  (params (OverlappedComponent :type "PrimitiveComponent Object Reference") (OtherActor :type "Actor Object Reference") (OtherComp :type "PrimitiveComponent Object Reference") (OtherBodyIndex :type Integer) (bFromSweep :type Boolean) (SweepResult :type "HitResult Structure (by ref)"))
  (cast `/Game/Blueprints/BP_Player` OtherActor) ; Check for player
  (bind _asbp_game_mode (cast `/Game/Blueprints/BP_GameMode` (`GameplayStatics.GetGameMode`)))
  ;[1 1 1] Add level part and increase score
  (`/Game/Blueprints/BP_GameMode.AddLevelPart` _asbp_game_mode)
  (`/Game/Blueprints/BP_GameMode.IncreaseScore` _asbp_game_mode 50)
  (`KismetSystemLibrary.Delay` 2.0)
  (`self.K2_DestroyActor`))

(fn `FindAttachPoint`
  (returns (AttachTransform :type "Transform Structure"))
  ;[0 1 0] Find attach point at end of level part
  (return (`SceneComponent.K2_GetComponentToWorld` (`self.AttachPoint`))))

(fn `UserConstructionScript`
  (`AddComponent|NODE_AddChildActorComponent-2` :`RelativeTransform` (`KismetMathLibrary.Conv_VectorToTransform` (`SceneComponent.RelativeLocation` (`self.EnemySpawnPoint`)))))
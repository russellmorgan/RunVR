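; BP_Player is a VR player actor that travels forward automatically and fires projectiles from both motion controllers.
; Each tick, it offsets itself along its forward vector by LevelSpeed read from BP_GameMode, scaled by delta time, without sweep.
; The left and right shoot inputs spawn BP_Projectile at the matching controller's location and rotation.
; BeginPlay sets a floor tracking origin for Oculus height, and a temporary Restart input reloads the Main level.
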(event `InputAction|ProjectileShootRight`
  (params (Key :type "Key Structure"))
  ;[1 1 1] Player shooting actions
  (:`Pressed`
    (`self.MotionControllerShoot` 0)))

(event `self.ReceiveTick`
  (params (DeltaSeconds :type "Float (single-precision)"))
  ;[0 1 0] Player moves forward
  (bind _output_get (set `self.DeltaSeconds` DeltaSeconds))
  (`self.PlayerMovement` _output_get))

(event `InputAction|ProjectileShootLeft`
  (params (Key :type "Key Structure"))
  ;[1 1 1] Player shooting actions
  (:`Pressed`
    (`self.MotionControllerShoot` 1)))

(event `self.ReceiveBeginPlay`
  ;[1 1 0] Set correct height for Oculus
  (`HeadMountedDisplayFunctionLibrary.SetTrackingOrigin` "Floor"))

(event `InputAction|Restart`
  (params (Key :type "Key Structure"))
  ;[1 1 0] temporary for testing
  (:`Pressed`
    (`GameplayStatics.OpenLevel` "Main")))

(fn `MotionControllerShoot`
  (params (WhichTrigger :type Integer))
  (bind _motioncontrollerright (`self.MotionControllerRight`))
  (bind _motioncontrollerleft (`self.MotionControllerLeft`))
  (switch `int` WhichTrigger ; Right = 0, left = 1
    (:`0`
      (`|SpawnActorFromClass` "/Game/Blueprints/BP_Projectile.BP_Projectile_C" (`KismetMathLibrary.MakeTransform` (`SceneComponent.K2_GetComponentLocation` _motioncontrollerright) (`SceneComponent.K2_GetComponentRotation` _motioncontrollerright)) "Undefined" "OverrideRootScale" null null))
    (:`1`
      (`|SpawnActorFromClass` "/Game/Blueprints/BP_Projectile.BP_Projectile_C" (`KismetMathLibrary.MakeTransform` (`SceneComponent.K2_GetComponentLocation` _motioncontrollerleft) (`SceneComponent.K2_GetComponentRotation` _motioncontrollerleft)) "Undefined" "OverrideRootScale" null null))))

(fn `PlayerMovement`
  (params (DeltaSeconds :type "Float (double-precision)"))
  (bind _asbp_game_mode (cast `/Game/Blueprints/BP_GameMode` (`GameplayStatics.GetGameMode`)))
  (set `self.DeltaSeconds` DeltaSeconds)
  (bind _output_get (set `self.PlayerMoveVector` (* (* (`self.GetActorForwardVector`) (`/Game/Blueprints/BP_GameMode.LevelSpeed` _asbp_game_mode)) (`self.DeltaSeconds`))))
  (`self.K2_AddActorWorldOffset` _output_get))

(fn `UserConstructionScript`)
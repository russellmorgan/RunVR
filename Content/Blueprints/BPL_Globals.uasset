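; Blueprint function library of shared hit responses for a scrolling shooter-style game.
; PlayerHitObstacle ends play on the game mode by clearing IsPlaying and zeroing LevelSpeed, then plays a hurt sound.
; EnemyHit sorts the overlapping actor by cast: a projectile is destroyed, plays the sound and adds score, while the player triggers PlayerHitObstacle.
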(fn `EnemyHit`
  (params (OtherActor :type "Actor Object Reference"))
  (bind _asbp_projectile (cast `/Game/Blueprints/BP_Projectile` OtherActor) ; Did a bullet hit the enemy?
    (:`then`
      (`Actor.K2_DestroyActor` _asbp_projectile)
      (`GameplayStatics.PlaySound2D` null "/Game/Retro_8Bit_Sounds/Damage_Hurt/Cues/retro_damage_hurt_ouch_07_Cue.retro_damage_hurt_ouch_07_Cue" 1.0 1.0 0.0 null null)
      (bind _asbp_game_mode (cast `/Game/Blueprints/BP_GameMode` (`GameplayStatics.GetGameMode` null)))
      (`/Game/Blueprints/BP_GameMode.IncreaseScore` _asbp_game_mode 1000))
    (:`CastFailed`
      (cast `/Game/Blueprints/BP_Player` OtherActor)
      (`self.PlayerHitObstacle` null))))

(fn `PlayerHitObstacle`
  (locals (finishedFade :type Boolean))
  (bind _asbp_game_mode (cast `/Game/Blueprints/BP_GameMode` (`GameplayStatics.GetGameMode` null)))
  (set `/Game/Blueprints/BP_GameMode.isPlaying` false _asbp_game_mode)
  (set `/Game/Blueprints/BP_GameMode.LevelSpeed` 0.0 _asbp_game_mode)
  (`GameplayStatics.PlaySound2D` null "/Game/Retro_8Bit_Sounds/Damage_Hurt/Cues/retro_damage_hurt_ouch_07_Cue.retro_damage_hurt_ouch_07_Cue" 1.0 1.0 0.0 null null))
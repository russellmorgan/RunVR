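; Game mode that builds a level from randomly chosen parts and tracks the game score.
; CreateInitialLevelParts, meant to be called from the level Blueprint, lays out the opening parts by repeatedly calling AddLevelPart.
; AddLevelPart spawns a random class from LevelPartsArray at NextSpawnPoint, then takes that part's attach point as the next spawn transform, chaining the parts.
; IncreaseScore adds to GameScore, while GameOver is an empty stub.
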(event `CreateInitialLevelParts`
  ;[0 1 0] Initial level part creation (call from level BP)
  (for _ (range 3)
    (`self.AddLevelPart`)))

(fn `AddLevelPart`
  (bind _levelpartsarray (`self.LevelPartsArray`))
  (bind _returnvalue (`|SpawnActorFromClass` (`|GetArrayItem` _levelpartsarray (`KismetMathLibrary.RandomIntegerInRange` 0 (`KismetArrayLibrary.Array_LastIndex` _levelpartsarray))) (`self.NextSpawnPoint`) "Undefined" "OverrideRootScale" null null))
  (bind _output_get (set `self.LevelPart` _returnvalue))
  (bind _asbp_level_part_base (cast `/Game/Blueprints/LevelParts/BP_LevelPart_Base` _output_get))
  (bind _attachtransform (`/Game/Blueprints/LevelParts/BP_LevelPart_Base.FindAttachPoint` _asbp_level_part_base))
  (set `self.NextSpawnPoint` _attachtransform))

(fn `GameOver`)

(fn `IncreaseScore`
  (params (ScoreValue :type Integer))
  (set `self.GameScore` (+ (`self.GameScore`) ScoreValue)))

(fn `UserConstructionScript`)